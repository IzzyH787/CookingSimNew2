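; BP_Oven is an interactable oven that cooks chicken items into BP_MadeStock counts.
; Interact opens WB_Oven once, switches to UI-only input and zeroes player walk speed.
; Tick polls CookingItem to start a real-time timer, then adds a per-item batch and resets.
; The timer check (CookTime >= elapsed) is inverted, completing cooks almost immediately; GetPortion and StartCook are stubs.
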(event EventTick
  (params (DeltaSeconds :type Float%20%28single-precision%29))
  ;[1 1 1] Checki if cooking
  (if (Variables|Default|GetCooking?)
    ;[1 1 1] Check if cooking timer has finished
    (if (>= (Variables|Default|GetcookTime) (- (Utilities|Time|GetRealTimeSeconds) (Variables|Default|GettimeStartedCooking)))
      ;[1 1 1] Update cooking states
      (Variables|Default|SetCooking? false)
      (Variables|Default|SetcookTime 0.0)
      (bind _returnvalue (Actor|GetActorOfClass "/Game/Blueprints/Non-physical/BP_MadeStock.BP_MadeStock_C"))
      (Utilities|FlowControl|Sequence
        (:then_0
          ;[1 1 1] Check what food is being cooked
          (if (== (Variables|Default|GetcookingItem) "Chicken")
            ;[1 1 1] Update stock levels
            (Variables|/Game/Blueprints/Non-physical/BP_MadeStock.BP_MadeStock_C|SetSpatchcock _returnvalue (+ (Variables|/Game/Blueprints/Non-physical/BP_MadeStock.BP_MadeStock_C|GetSpatchcock _returnvalue) 12))
            ;[1 1 1] Reset item being cooked
            (Variables|Default|SetcookingItem "None" :!label _label)))
        (:then_1
          (if (== (Variables|Default|GetcookingItem) "Butterfly")
            (Variables|/Game/Blueprints/Non-physical/BP_MadeStock.BP_MadeStock_C|SetButterfly _returnvalue (+ (Variables|/Game/Blueprints/Non-physical/BP_MadeStock.BP_MadeStock_C|GetButterfly _returnvalue) 15))
            (goto _label)))
        (:then_2
          (if (== (Variables|Default|GetcookingItem) "Thighs")
            (Variables|/Game/Blueprints/Non-physical/BP_MadeStock.BP_MadeStock_C|SetThighs _returnvalue (+ (Variables|/Game/Blueprints/Non-physical/BP_MadeStock.BP_MadeStock_C|GetThighs _returnvalue) 40))
            (goto _label)))
        (:then_3
          (if (== (Variables|Default|GetcookingItem) "Wings")
            (Variables|/Game/Blueprints/Non-physical/BP_MadeStock.BP_MadeStock_C|SetWings _returnvalue (+ (Variables|/Game/Blueprints/Non-physical/BP_MadeStock.BP_MadeStock_C|GetWings _returnvalue) 40))
            (goto _label)))))
    (else
      (Utilities|FlowControl|Sequence
        (:then_0
          ;[1 1 1] Check food being cooked
          (if (== (Variables|Default|GetcookingItem) "Chicken")
            ;[1 1 1] Set cooking timer
            (Variables|Default|SetcookTime 6e+01)
            (Variables|Default|SetCooking? true :!label _label_2)
            ;[1 1 1] Capture time started cooking
            (Variables|Default|SettimeStartedCooking (Utilities|Time|GetRealTimeSeconds))))
        (:then_1
          (if (== (Variables|Default|GetcookingItem) "Butterfly")
            (Variables|Default|SetcookTime 45.0 :!label _label_3)
            (goto _label_2)))
        (:then_2
          (if (== (Variables|Default|GetcookingItem) "Thighs")
            (goto _label_3)))
        (:then_3
          (if (== (Variables|Default|GetcookingItem) "Wings")
            (goto _label_3)))))))

(fn ConstructionScript
  (Variables|Default|SetcookTime 0.0)
  (Variables|Default|SetCooking? false)
  (Variables|Default|SetUIOpen? false))

(fn GetPortion
  (params (Interactor :type Character%20Event%20Structure))
  (return false))

(fn Interact
  (params (Interactor :type Character%20Event%20Structure))
  (bind _returnvalue (Game|GetPlayerController 0))
  ;[1 1 1] Check if UI is already opened
  (if (not (Variables|Default|GetUIOpen?))
    ;[1 1 1] Make widget visible
    (bind _returnvalue_2 (UserInterface|CreateWidget "/Game/UI/WB_Oven.WB_Oven_C"))
    (UserInterface|Viewport|AddtoViewport _returnvalue_2 0)
    ;[1 1 1] Turn off player controls
    (Variables|/Script/Engine.PlayerController|SetbShowMouseCursor _returnvalue true)
    (Input|SetInputModeUIOnly _returnvalue 0 "DoNotLock" false)
    (Variables|Default|SetUIOpen? true)
    ;[1 1 1] Stop player moving
    (bind _returnvalue_3 (Actor|GetActorOfClass "/Game/Characters/Blueprints/BP_Player.BP_Player_C"))
    (Variables|/Script/Engine.CharacterMovementComponent|SetMaxWalkSpeed (Variables|/Script/Engine.Character|GetCharacterMovement _returnvalue_3) 0.0)
    (return true)))

(fn StartCook
  (params (Interactor :type Character%20Event%20Structure))
  (return false))