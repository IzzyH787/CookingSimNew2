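; Interactable fryer that cooks timed batches of chips and holds the portions for scooping into stock.
; Interact opens the WB_Fryer UI, switches to UI-only input and stops player movement, while a box overlap shows the world widget and timer text.
; StartCook records a real-time start, Tick updates the countdown and adds portions when it expires, and GetPortion scoops one into BP_MadeStock's Fries count.
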(event OnComponentBeginOverlap(Box)
  (params (OverlappedComponent :type Primitive%20Component%20Object%20Reference) (OtherActor :type Actor%20Object%20Reference) (OtherComp :type Primitive%20Component%20Object%20Reference) (OtherBodyIndex :type Integer) (bFromSweep :type Boolean) (SweepResult :type Hit%20Result%20Structure%20%28by%20ref%29))
  (Development|SetHiddeninGame (Variables|Default|GetWidget) false false)
  (Development|SetHiddeninGame (Variables|Default|GetTimeRemaining) false false))

(event OnComponentEndOverlap(Box)
  (params (OverlappedComponent :type Primitive%20Component%20Object%20Reference) (OtherActor :type Actor%20Object%20Reference) (OtherComp :type Primitive%20Component%20Object%20Reference) (OtherBodyIndex :type Integer))
  (Development|SetHiddeninGame (Variables|Default|GetWidget) true false)
  (Development|SetHiddeninGame (Variables|Default|GetTimeRemaining) true false))

(event EventTick
  (params (DeltaSeconds :type Float%20%28single-precision%29))
  (if (Variables|Default|GetisCooking)
    (bind _text (CallFunction|PrintTimer))
    (Rendering|Components|TextRender|SetText (Variables|Default|GetTimeRemaining) _text)
    ;[1 1 1] Check if fryer has been cooking long enough to stop
    (if (>= (- (Utilities|Time|GetRealTimeSeconds) (Variables|Default|GettimeCookStarted)) (Variables|Default|Gettimer))
      (Rendering|Components|TextRender|SetText (Variables|Default|GetTimeRemaining) (Utilities|Text|MakeLiteralText "Empty"))
      (Variables|Default|SetisCooking false)
      ;[1 1 1] Update how many portions are now held in the fryer
      (Variables|Default|SetportionsHeld (+ (Variables|Default|GetportionsHeld) 5.0))
      (Development|PrintString (Utilities|String|ToString(Float) (Variables|Default|GetportionsHeld))))))

(fn ConstructionScript)

(fn UseFryer
  (Development|PrintString "Test")
  (Variables|Default|SetisInteractable (Class|KismetSystemLibrary|MakeLiteralBool true))
  (Development|PrintString (Utilities|String|ToString(Boolean) (Variables|Default|GetisInteractable))))

(fn Cook
  (if (not (Variables|Default|GetisCooking))
    (Variables|Default|SettimeCookStarted (Utilities|Time|GetRealTimeSeconds))
    (Variables|Default|SetisCooking true)
    (bind _output_get (Variables|Default|Settimer 6e+01))
    (Development|PrintString (Utilities|String|ToString(Float) _output_get))))

(fn Scoop
  (if (> (Variables|Default|GetportionsHeld) 0.0)
    ;[1 1 1] Decrease num of portions held in fryer
    (Variables|Default|SetportionsHeld (- (Variables|Default|GetportionsHeld) 1.0))
    ;[1 1 1] Increment stock
    (bind _returnvalue (Actor|GetActorOfClass "/Game/Blueprints/Non-physical/BP_MadeStock.BP_MadeStock_C"))
    (Variables|/Game/Blueprints/Non-physical/BP_MadeStock.BP_MadeStock_C|SetFries _returnvalue (+ (Variables|/Game/Blueprints/Non-physical/BP_MadeStock.BP_MadeStock_C|GetFries _returnvalue) 10))
    (else
      (Development|PrintString "No chips!"))))

(fn PrintTimer
  (bind _returnvalue (Utilities|Time|GetRealTimeSeconds))
  (bind _timer (Variables|Default|Gettimer))
  (bind _timecookstarted (Variables|Default|GettimeCookStarted))
  (bind _returnvalue_2 (- _returnvalue _timecookstarted))
  (bind _returnvalue_3 (- _timer _returnvalue_2))
  (bind _returnvalue_4 (/ _returnvalue_3 6e+01))
  (bind _returnvalue_5 (Math|Float|Truncate _returnvalue_4))
  (bind _returnvalue_6 (Utilities|String|ToString(Integer) _returnvalue_5))
  (bind _returnvalue_7 (* _returnvalue_5 60))
  (bind _returnvalue_8 (- _returnvalue_3 _returnvalue_7))
  (bind _returnvalue_9 (Math|Float|Truncate _returnvalue_8))
  (bind _returnvalue_10 (Utilities|String|ToString(Integer) _returnvalue_9))
  (if (>= _returnvalue_9 10)
    (return (Utilities|Text|ToText(String) (Utilities|String|Append "Time Remaining: " _returnvalue_6 ":" _returnvalue_10)))
    (else
      (return (Utilities|Text|ToText(String) (Utilities|String|Append "Time Remaining: " _returnvalue_6 ":0" _returnvalue_10))))))

(fn GetPortion
  (params (Interactor :type Character%20Event%20Structure))
  (CallFunction|Scoop)
  (return false))

(fn Interact
  (params (Interactor :type Character%20Event%20Structure))
  (bind _returnvalue (Game|GetPlayerController 0))
  ;[1 1 1] checks multiple UIs won't be opened
  (if (not (Variables|Default|GetUIOpen?))
    ;[1 1 1] Open UI onto screen
    (bind _returnvalue_2 (UserInterface|CreateWidget "/Game/UI/WB_Fryer.WB_Fryer_C"))
    (UserInterface|Viewport|AddtoViewport _returnvalue_2 0)
    ;[1 1 1] Turn off player controls
    (Variables|/Script/Engine.PlayerController|SetbShowMouseCursor _returnvalue true)
    (Input|SetInputModeUIOnly _returnvalue _returnvalue_2 "DoNotLock" false)
    ;[1 1 1] Acknowledge UI is now open
    (Variables|Default|SetUIOpen? true)
    ;[1 1 1] Stop player moving
    (bind _returnvalue_3 (Actor|GetActorOfClass "/Game/Characters/Blueprints/BP_Player.BP_Player_C"))
    (Variables|/Script/Engine.CharacterMovementComponent|SetMaxWalkSpeed (Variables|/Script/Engine.Character|GetCharacterMovement _returnvalue_3) 0.0)
    (return true)))

(fn StartCook
  (params (Interactor :type Character%20Event%20Structure))
  (CallFunction|Cook)
  (return false))