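; BP_FrontGrill is an interactable front grill that opens its own CAW_FrontGrill UI.
; An overlap area shows or hides the prompt widget, while Interact adds and activates the UI created at BeginPlay, then enables the cursor with Game and UI input.
; A UIOpen flag blocks reopening and is never cleared here.
; GetPortion and StartCook only return false, and Delay is a countdown loop that does not wait in real time.
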(event OnComponentBeginOverlap(InteractArea)
  (params (OverlappedComponent :type Primitive%20Component%20Object%20Reference) (OtherActor :type Actor%20Object%20Reference) (OtherComp :type Primitive%20Component%20Object%20Reference) (OtherBodyIndex :type Integer) (bFromSweep :type Boolean) (SweepResult :type Hit%20Result%20Structure%20%28by%20ref%29))
  ;[1 1 1] Show interact prompt when player in range to interact
  (Development|SetHiddeninGame (Variables|Default|GetWidget) false false))

(event OnComponentEndOverlap(InteractArea)
  (params (OverlappedComponent :type Primitive%20Component%20Object%20Reference) (OtherActor :type Actor%20Object%20Reference) (OtherComp :type Primitive%20Component%20Object%20Reference) (OtherBodyIndex :type Integer))
  ;[1 1 1] Hide UI when player leaves range they can interact
  (Development|SetHiddeninGame (Variables|Default|GetWidget) true false))

(event EventBeginPlay
  ;[1 1 1] Create UI widget
  (bind _returnvalue (UserInterface|CreateWidget "/Game/UI/CAW_FrontGrill.CAW_FrontGrill_C"))
  (Variables|Default|SetUI _returnvalue))

(fn ConstructionScript)

(fn Delay
  (params (delayTime :type Float%20%28double-precision%29))
  (Variables|Default|SetdelayTimer delayTime)
  ;[1 1 1] While time in delay > 0
  (while (> (Variables|Default|GetdelayTimer) 0.0)
    ;[1 1 1] Decrement timer
    (Variables|Default|SetdelayTimer (- (Variables|Default|GetdelayTimer) 1.0)))
  (Development|PrintString "Delay over"))

(fn GetPortion
  (params (Interactor :type Character%20Event%20Structure))
  (return false))

(fn Interact
  (params (Interactor :type Character%20Event%20Structure))
  (bind _returnvalue (Game|GetPlayerController 0))
  (bind _ui (Variables|Default|GetUI))
  (if (not (Variables|Default|GetUIOpen))
    (UserInterface|Viewport|AddtoViewport _ui 0)
    (Class|CommonActivatableWidget|ActivateWidget _ui)
    ;[1 1 1] Turn off player controls
    (Variables|/Script/Engine.PlayerController|SetbShowMouseCursor _returnvalue true)
    (Input|SetInputModeGameandUI _returnvalue 0 "DoNotLock" true false)
    (Variables|Default|SetUIOpen true)
    (return false)))

(fn StartCook
  (params (Interactor :type Character%20Event%20Structure))
  (return false))