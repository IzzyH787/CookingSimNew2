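; BP_CoordScreen is an interactable screen actor that brings up the WB_CoordScreen widget in the viewport.
; Interact creates and adds the widget when UIOpen is false, though UIOpen is never set in these graphs.
; GetPortion and StartCook are stubs returning false.
; DisplayOrders only gathers all BP_Order actors without using the result, and the event graph is empty apart from disabled default events.
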(event EventBeginPlay)

(event Collision|EventActorBeginOverlap
  (params (OtherActor :type Actor%20Object%20Reference)))

(event EventTick
  (params (DeltaSeconds :type Float%20%28single-precision%29)))

(fn ConstructionScript)

(fn DisplayOrders
  (Actor|GetAllActorsOfClass "/Game/Blueprints/BP_Order.BP_Order_C"))

(fn GetPortion
  (params (Interactor :type Character%20Event%20Structure))
  (return false))

(fn Interact
  (params (Interactor :type Character%20Event%20Structure))
  (if (not (Variables|Default|GetUIOpen?))
    (bind _returnvalue (UserInterface|CreateWidget "/Game/UI/WB_CoordScreen.WB_CoordScreen_C"))
    (UserInterface|Viewport|AddtoViewport _returnvalue 0)
    (return false)))

(fn StartCook
  (params (Interactor :type Character%20Event%20Structure))
  (return false))