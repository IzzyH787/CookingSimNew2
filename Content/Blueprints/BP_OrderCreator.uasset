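; BP_OrderCreator is a spawner actor that creates BP_Order actors at its own transform at random intervals.
; Tick advances a counter by one per frame rather than by delta time, so intervals are measured in frames and vary with framerate.
; When the count since the last spawn reaches NextDelay, it spawns an order, rolls a new delay between MinDelay and MaxDelay, and prints a debug message.
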(event EventBeginPlay
  (Variables|Default|SetminDelay 1e+03)
  (Variables|Default|SetmaxDelay 2e+03)
  (Variables|Default|SetcurrentTime 0.0)
  (Variables|Default|SetlastCreation 0.0)
  (CallFunction|GenerateNextDelay))

(event EventTick
  (params (DeltaSeconds :type Float%20%28single-precision%29))
  ;[1 1 1] Increment Timer
  (Variables|Default|SetcurrentTime (+ (Variables|Default|GetcurrentTime) 1.0))
  ;[1 1 1] Check if enough time has passed to spawn a new order
  (if (>= (- (Variables|Default|GetcurrentTime) (Variables|Default|GetlastCreation)) (Variables|Default|GetnextDelay))
    (Game|SpawnActorfromClass "/Game/Blueprints/BP_Order.BP_Order_C" (Transformation|GetActorTransform) "Undefined" "MultiplyWithRoot" 0 0)
    (CallFunction|GenerateNextDelay)
    (Variables|Default|SetlastCreation (Variables|Default|GetcurrentTime))
    (Development|PrintString "Order ")))

(fn ConstructionScript)

(fn GenerateNextDelay
  (Variables|Default|SetnextDelay (Math|Random|RandomFloatinRange (Variables|Default|GetminDelay) (Variables|Default|GetmaxDelay))))