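; BP_Chicken is a chicken food item that cooks and then burns over time.
; The construction script timestamps TimeOnGrill with real time and derives the burn threshold from cook time plus a burn delay.
; Tick compares elapsed time to both thresholds, updating the Cooked and Burnt flags and swapping the Cube's material.
; The timer runs from construction, with no check for actual grill contact.
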(event EventTick
  (params (DeltaSeconds :type Float%20%28single-precision%29))
  ;[1 1 1] Check if cooked
  (if (>= (- (Utilities|Time|GetRealTimeSeconds) (Variables|Default|GettimeOnGrill)) (Variables|Default|GettimeUntilCooked))
    ;[1 1 1] Set to cooked, change material
    (Variables|Default|Setcooked? true)
    (Rendering|Material|SetMaterial (Variables|Default|GetCube) 0 "/DatasmithContent/Materials/AliasReference.AliasReference")
    ;[1 1 1] Check if burnt
    (if (>= (- (Utilities|Time|GetRealTimeSeconds) (Variables|Default|GettimeOnGrill)) (Variables|Default|GettimeUntilBurnt))
      (Variables|Default|Setcooked? false)
      ;[1 1 1] Set to burnt, change material
      (Variables|Default|Setburnt? true)
      (Rendering|Material|SetMaterial (Variables|Default|GetCube) 0 "/Engine/EngineDebugMaterials/BlackUnlitMaterial.BlackUnlitMaterial"))))

(fn ConstructionScript
  (Variables|Default|SettimeUntilCooked 1.2e+02)
  (Variables|Default|SettimeOnGrill (Utilities|Time|GetRealTimeSeconds))
  (Variables|Default|Setcooked? false)
  (Variables|Default|Setburnt? false)
  (Variables|Default|SetburnDelay 6e+01)
  (Variables|Default|SettimeUntilBurnt (+ (Variables|Default|GettimeUntilCooked) (Variables|Default|GetburnDelay))))