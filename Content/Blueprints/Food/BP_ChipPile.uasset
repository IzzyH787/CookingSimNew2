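; BP_ChipPile is a food prop that displays a pile of chips sized to a portion count.
; The mesh starts hidden in game on BeginPlay.
; CreatePile switches on Portions to swap between five pile meshes and show the result, hiding it again at zero and using the largest pile for any unlisted value.
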(event EventBeginPlay
  (Development|SetHiddeninGame (Variables|Default|GetStaticMesh) true false))

(fn ConstructionScript)

(fn CreatePile
  (params (Portions :type Integer))
  (bind _staticmesh (Variables|Default|GetStaticMesh))
  (bind _staticmesh_2 (Variables|Default|GetStaticMesh))
  (bind _staticmesh_3 (Variables|Default|GetStaticMesh))
  (bind _staticmesh_4 (Variables|Default|GetStaticMesh))
  (bind _staticmesh_5 (Variables|Default|GetStaticMesh))
  (bind _staticmesh_6 (Variables|Default|GetStaticMesh))
  (switch int Portions
    (:Default
      (Components|StaticMesh|SetStaticMesh _staticmesh "/Game/Assets/ChipPiles/ChipPile5.ChipPile5")
      (Development|SetHiddeninGame _staticmesh false false))
    (:0
      (Components|StaticMesh|SetStaticMesh _staticmesh_2 "/Game/Assets/ChipPiles/ChipPile1.ChipPile1")
      (Development|SetHiddeninGame _staticmesh_2 true false))
    (:1
      (Components|StaticMesh|SetStaticMesh _staticmesh_3 "/Game/Assets/ChipPiles/ChipPile1.ChipPile1")
      (Development|SetHiddeninGame _staticmesh_3 false false))
    (:2
      (Components|StaticMesh|SetStaticMesh _staticmesh_4 "/Game/Assets/ChipPiles/ChipPile2.ChipPile2")
      (Development|SetHiddeninGame _staticmesh_4 false false))
    (:3
      (Components|StaticMesh|SetStaticMesh _staticmesh_5 "/Game/Assets/ChipPiles/ChipPile3.ChipPile3")
      (Development|SetHiddeninGame _staticmesh_5 false false))
    (:4
      (Components|StaticMesh|SetStaticMesh _staticmesh_6 "/Game/Assets/ChipPiles/ChipPile4.ChipPile4")
      (Development|SetHiddeninGame _staticmesh_6 false false))))