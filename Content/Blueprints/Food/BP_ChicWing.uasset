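; BP_ChicWing is a chicken wing food Blueprint that models cooked and burnt states from time on the grill.
; The construction script records the real-time start and sets the cook threshold, with the burn threshold a fixed delay later.
; Logic comparing elapsed time to these thresholds sets state flags and swaps the Cube material.
; That logic is disconnected from the empty Tick event, so it never runs.
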(event EventTick
  (params (DeltaSeconds :type Float%20%28single-precision%29)))

(fn ConstructionScript
  (Variables|Default|SettimeUntilCooked 45.0)
  (Variables|Default|SettimeOnGrill (Utilities|Time|GetRealTimeSeconds))
  (Variables|Default|Setcooked? false)
  (Variables|Default|Setburnt? false)
  (Variables|Default|SetburnDelay 45.0)
  (Variables|Default|SettimeUntilBurnt (+ (Variables|Default|GettimeUntilCooked) (Variables|Default|GetburnDelay))))