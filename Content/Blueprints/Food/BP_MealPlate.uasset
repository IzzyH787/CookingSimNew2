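; BP_MealPlate is a food plate whose mesh shows the meal in a given order.
; AssignMeal stores the Order, then checks chicken, thighs, butterfly and wings in sequence, swapping the Plate static mesh for each match.
; Wings pick a platter by exact piece count, and other counts leave the mesh as is.
; Only one mesh shows, so the last matching check wins on mixed orders.
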(fn ConstructionScript)

(fn AssignMeal
  (params (Order :type BP%20Order%20Object%20Reference))
  (Variables|Default|SetOrder Order)
  (Utilities|FlowControl|Sequence
    (:then_0
      ;[1 1 1] Check if chicken on order
      (if (> (Variables|/Game/Blueprints/Non-physical/BP_Order.BP_Order_C|GetChicken (Variables|Default|GetOrder)) 0)
        ;[1 1 1] Setting static mesh of plate
        (Components|StaticMesh|SetStaticMesh (Variables|Default|GetPlate) "/Game/Assets/PlatedFood/Chicken/ChickenPlate.ChickenPlate")))
    (:then_1
      ;[1 1 1] Check if thighs on order
      (if (> (Variables|/Game/Blueprints/Non-physical/BP_Order.BP_Order_C|GetThighs (Variables|Default|GetOrder)) 0)
        (Components|StaticMesh|SetStaticMesh (Variables|Default|GetPlate) "/Game/Assets/PlatedFood/Thighs/ThighPlate.ThighPlate")))
    (:then_2
      ;[1 1 1] Check if butterfly on order
      (if (> (Variables|/Game/Blueprints/Non-physical/BP_Order.BP_Order_C|GetButterfly (Variables|Default|GetOrder)) 0)
        (Components|StaticMesh|SetStaticMesh (Variables|Default|GetPlate) "/Game/Assets/PlatedFood/Butterfly/ButterflyPlate.ButterflyPlate")))
    (:then_3
      ;[1 1 1] Check if wings on order
      (switch int (Variables|/Game/Blueprints/Non-physical/BP_Order.BP_Order_C|GetWings (Variables|Default|GetOrder))
        (:3
          (Components|StaticMesh|SetStaticMesh (Variables|Default|GetPlate) "/Game/Assets/PlatedFood/Wings/3/3WingPlatter.3WingPlatter"))
        (:5
          (Components|StaticMesh|SetStaticMesh (Variables|Default|GetPlate) "/Game/Assets/PlatedFood/Wings/5/5WingPlatter.5WingPlatter"))
        (:10
          (Components|StaticMesh|SetStaticMesh (Variables|Default|GetPlate) "/Game/Assets/PlatedFood/Wings/10/10WingPlate.10WingPlate"))
        (:15
          (Components|StaticMesh|SetStaticMesh (Variables|Default|GetPlate) "/Game/Assets/PlatedFood/Wings/15/15WingPlate.15WingPlate"))))))