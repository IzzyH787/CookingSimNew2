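; Front door actor that opens for non-player actors and shows a leave-level menu when the player enters its trigger box.
; On BeginPlay it creates the CAW_LeaveLevel widget, which a Player-tagged overlap activates while switching to UI-only input, showing the cursor and pausing the game.
; Other overlapping actors play a timeline that drives the door's yaw, and any end overlap reverses it.
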(event OnComponentBeginOverlap(Box)
  (params (OverlappedComponent :type Primitive%20Component%20Object%20Reference) (OtherActor :type Actor%20Object%20Reference) (OtherComp :type Primitive%20Component%20Object%20Reference) (OtherBodyIndex :type Integer) (bFromSweep :type Boolean) (SweepResult :type Hit%20Result%20Structure%20%28by%20ref%29))
  (bind _returnvalue (Game|GetPlayerController 0))
  (bind _leavelevelui (Variables|Default|GetLeaveLevelUI))
  (if (Actor|ActorHasTag OtherActor "Player")
    (UserInterface|Viewport|AddtoViewport _leavelevelui 0)
    (Class|CommonActivatableWidget|ActivateWidget _leavelevelui)
    (Input|SetInputModeUIOnly _returnvalue 0 "DoNotLock" false)
    (Variables|/Script/Engine.PlayerController|SetbShowMouseCursor _returnvalue true)
    (Game|SetGamePaused true)
    (else
      (bind _doorrotationz (Timeline|DoorTimelineComponent Play)
        (:Update
          (Transformation|SetRelativeRotation (Variables|Default|GetDoor) (Math|Rotator|MakeRotator 0.0 0.0 _doorrotationz) false false))))))

(event OnComponentEndOverlap(Box)
  (params (OverlappedComponent :type Primitive%20Component%20Object%20Reference) (OtherActor :type Actor%20Object%20Reference) (OtherComp :type Primitive%20Component%20Object%20Reference) (OtherBodyIndex :type Integer))
  (bind _doorrotationz (Timeline|DoorTimelineComponent Reverse)
    (:Update
      (Transformation|SetRelativeRotation (Variables|Default|GetDoor) (Math|Rotator|MakeRotator 0.0 0.0 _doorrotationz) false false))))

(event EventBeginPlay
  (bind _returnvalue (UserInterface|CreateWidget "/Game/UI/CAW_LeaveLevel.CAW_LeaveLevel_C"))
  (Variables|Default|SetLeaveLevelUI _returnvalue))

(fn ConstructionScript)