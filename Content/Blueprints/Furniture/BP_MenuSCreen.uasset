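; BP_MenuSCreen is a furniture screen prop that periodically glitches between a normal menu display and a broken look.
; On Tick it compares real time against a random delay and toggles the screen's material between M_MenuScreen and M_HLSLShader.
; Two helper functions pick the delays, so the screen stays working much longer than it stays broken.
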(event EventTick
  (params (DeltaSeconds :type Float%20%28single-precision%29))
  (if (>= (- (Utilities|Time|GetRealTimeSeconds) (Variables|Default|GetlastTimeScreenChanged)) (Variables|Default|GetchangeDelay))
    (Variables|Default|SetlastTimeScreenChanged (Utilities|Time|GetRealTimeSeconds))
    (if (Variables|Default|GetscreenIsBroken?)
      (Rendering|Material|SetMaterial (Variables|Default|GetScreen) 0 "/Game/Materials/M_MenuScreen.M_MenuScreen")
      (bind _nextbreakdelay (CallFunction|GenerateNextBreakDelay))
      (Variables|Default|SetchangeDelay _nextbreakdelay)
      (Variables|Default|SetscreenIsBroken? false)
      (else
        (Rendering|Material|SetMaterial (Variables|Default|GetScreen) 0 "/Game/Materials/M_HLSLShader.M_HLSLShader")
        (bind _delayuntilfixed (CallFunction|GenerateDelayUntilFixed))
        (Variables|Default|SetchangeDelay _delayuntilfixed)
        (Variables|Default|SetscreenIsBroken? true)))))

(event EventBeginPlay
  (Variables|Default|SetscreenIsBroken? false)
  (Rendering|Material|SetMaterial (Variables|Default|GetScreen) 0 "/Game/Materials/M_MenuScreen.M_MenuScreen")
  (bind _nextbreakdelay (CallFunction|GenerateNextBreakDelay))
  (Variables|Default|SetchangeDelay _nextbreakdelay))

(fn ConstructionScript)

(fn GenerateNextBreakDelay
  (return (Math|Random|RandomFloatinRange 15.0 25.0)))

(fn GenerateDelayUntilFixed
  (return (Math|Random|RandomFloatinRange 5.0 8.0)))