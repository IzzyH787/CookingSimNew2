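; Timed spawner that feeds new customers and their orders into the restaurant while it is not full.
; Tick compares real time since the last spawn against a random interval rerolled by GenerateNextDelay after each spawn.
; When due, it spawns an AI customer at the customer spawner and registers it in the level manager's CustomerList.
; After a fixed Delay, it spawns a BP_Order at its own transform and stores it in OrderList.
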(event EventBeginPlay
  ;[1 1 1] Initialise variables
  (Variables|Default|SetminDelay 15.0)
  (Variables|Default|SetmaxDelay 2e+01)
  (Variables|Default|SetcurrentTime 0.0)
  (Variables|Default|SetlastCreation 0.0)
  ;[1 1 1] Create wait until next order
  (CallFunction|GenerateNextDelay))

(event EventTick
  (params (DeltaSeconds :type Float%20%28single-precision%29))
  ;[1 1 1] Check if restuarant is not full
  (bind _returnvalue (Actor|GetActorOfClass "/Game/Blueprints/Non-physical/BP_LevelManager.BP_LevelManager_C"))
  (if (not (Variables|/Game/Blueprints/Non-physical/BP_LevelManager.BP_LevelManager_C|GetrestaurantFull? _returnvalue))
    ;[1 1 1] Check if enough time has passed to spawn a new order
    (if (>= (- (Utilities|Time|GetRealTimeSeconds) (Variables|Default|GetlastCreation)) (Variables|Default|GetnextDelay))
      ;[1 1 1] Spawn customer
      (bind _returnvalue_2 (Actor|GetActorOfClass "/Game/Blueprints/Non-physical/BP_CustomerSpawner.BP_CustomerSpawner_C"))
      (bind _returnvalue_3 (AI|SpawnAIFromClass "/Game/Characters/CustomerAI/BP_CustomerAI.BP_CustomerAI_C" 0 (Math|Vector|MakeVector (.x (Transformation|GetActorLocation _returnvalue_2)) (.y (Transformation|GetActorLocation _returnvalue_2)) 4e+02) "0, 0, 0" false 0))
      ;[1 1 1] Add new customer to list of customers
      (bind _asbp_customer_ai (Utilities|Casting|CastToBP_CustomerAI _returnvalue_3))
      (bind _returnvalue_4 (Actor|GetActorOfClass "/Game/Blueprints/Non-physical/BP_LevelManager.BP_LevelManager_C"))
      (Utilities|Array|Add (Variables|/Game/Blueprints/Non-physical/BP_LevelManager.BP_LevelManager_C|GetcustomerList _returnvalue_4) _asbp_customer_ai)
      (CallFunction|GenerateNextDelay)
      ;[1 1 1] Change last creation time
      (Variables|Default|SetlastCreation (Utilities|Time|GetRealTimeSeconds))
      (Utilities|FlowControl|Delay 17.0)
      ;[1 1 1] Create order
      (bind _returnvalue_5 (Game|SpawnActorfromClass "/Game/Blueprints/Non-physical/BP_Order.BP_Order_C" (Transformation|GetActorTransform) "AlwaysSpawn" "MultiplyWithRoot" 0 0))
      (Utilities|Array|Add (Variables|Default|GetOrderList) _returnvalue_5)
      (Development|PrintString "Customer spawned"))))

(fn ConstructionScript)

(fn GenerateNextDelay
  (Variables|Default|SetnextDelay (Math|Random|RandomFloatinRange (Variables|Default|GetminDelay) (Variables|Default|GetmaxDelay))))