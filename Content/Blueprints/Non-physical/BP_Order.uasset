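; BP_Order represents a randomly generated food order, with item quantities, a creation timestamp and a text summary.
; The Construction Script records real time, randomises Chicken, Thighs, Butterfly and Fries, and leaves other items at their existing values.
; It then appends each item with a count above zero to OrderList, using CheckOnOrder.
; The EventGraph holds an unreached copy of this logic, and CreateOrder is an empty stub.
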(fn ConstructionScript
  (Variables|Default|SettimeOfCreation (Utilities|Time|GetRealTimeSeconds))
  ;[1 1 1] Setting values of each item on order
  (Variables|Default|SetmaxRange 5)
  (Variables|Default|SetChicken (Math|Random|RandomIntegerinRange 0 (Variables|Default|GetmaxRange)))
  (Variables|Default|SetThighs (Math|Random|RandomIntegerinRange 0 (Variables|Default|GetmaxRange)))
  (Variables|Default|SetButterfly (Math|Random|RandomIntegerinRange 0 (Variables|Default|GetmaxRange)))
  (Variables|Default|SetFries (Math|Random|RandomIntegerinRange 1 5))
  (Utilities|FlowControl|Sequence
    (:then_0
      ;[1 1 1] Check if item is on order
      (bind _onorder_ (CallFunction|CheckonOrder (Variables|Default|GetThighs)))
      ;[1 1 1] If item on order, add it to the text list
      (if _onorder_
        (Variables|Default|SetOrderList (Utilities|String|Append (Variables|Default|GetOrderList) (Utilities|String|Append (Utilities|String|MakeLiteralString "Thighs ") (Utilities|String|ToString(Integer) (Variables|Default|GetThighs)))))
        (Variables|Default|SetOrderList (Utilities|String|Append (Variables|Default|GetOrderList) " 
") :!label _label)))
    (:then_1
      (bind _onorder__2 (CallFunction|CheckonOrder (Variables|Default|GetChicken)))
      (if _onorder__2
        (Variables|Default|SetOrderList (Utilities|String|Append (Variables|Default|GetOrderList) (Utilities|String|Append (Utilities|String|MakeLiteralString "Chicken") (Utilities|String|ToString(Integer) (Variables|Default|GetChicken)))))
        (goto _label)))
    (:then_2
      (bind _onorder__3 (CallFunction|CheckonOrder (Variables|Default|GetButterfly)))
      (if _onorder__3
        (Variables|Default|SetOrderList (Utilities|String|Append (Variables|Default|GetOrderList) (Utilities|String|Append (Utilities|String|MakeLiteralString "Butterfly ") (Utilities|String|ToString(Integer) (Variables|Default|GetButterfly)))))
        (goto _label)))
    (:then_3
      (bind _onorder__4 (CallFunction|CheckonOrder (Variables|Default|GetBurger)))
      (if _onorder__4
        (Variables|Default|SetOrderList (Utilities|String|Append (Variables|Default|GetOrderList) (Utilities|String|Append (Utilities|String|MakeLiteralString "Burger") (Utilities|String|ToString(Integer) (Variables|Default|GetBurger)))))
        (goto _label)))
    (:then_4
      (bind _onorder__5 (CallFunction|CheckonOrder (Variables|Default|GetWrap)))
      (if _onorder__5
        (Variables|Default|SetOrderList (Utilities|String|Append (Variables|Default|GetOrderList) (Utilities|String|Append (Utilities|String|MakeLiteralString "Wrap") (Utilities|String|ToString(Integer) (Variables|Default|GetWrap)))))
        (goto _label)))
    (:then_5
      (bind _onorder__6 (CallFunction|CheckonOrder (Variables|Default|GetFries)))
      (if _onorder__6
        (Variables|Default|SetOrderList (Utilities|String|Append (Variables|Default|GetOrderList) (Utilities|String|Append (Utilities|String|MakeLiteralString "Fries") (Utilities|String|ToString(Integer) (Variables|Default|GetFries)))))
        (goto _label)))
    (:then_6
      (bind _onorder__7 (CallFunction|CheckonOrder (Variables|Default|GetPeriFries)))
      (if _onorder__7
        (Variables|Default|SetOrderList (Utilities|String|Append (Variables|Default|GetOrderList) (Utilities|String|Append (Utilities|String|MakeLiteralString "Peri Fries") (Utilities|String|ToString(Integer) (Variables|Default|GetPeriFries)))))
        (goto _label)))
    (:then_7
      (bind _onorder__8 (CallFunction|CheckonOrder (Variables|Default|GetMash)))
      (if _onorder__8
        (Variables|Default|SetOrderList (Utilities|String|Append (Variables|Default|GetOrderList) (Utilities|String|Append (Utilities|String|MakeLiteralString "Mash") (Utilities|String|ToString(Integer) (Variables|Default|GetMash)))))
        (goto _label)))
    (:then_8
      (bind _onorder__9 (CallFunction|CheckonOrder (Variables|Default|GetWings)))
      (if _onorder__9
        (Variables|Default|SetOrderList (Utilities|String|Append (Variables|Default|GetOrderList) (Utilities|String|Append (Utilities|String|MakeLiteralString "Wings") (Utilities|String|ToString(Integer) (Variables|Default|GetWings)))))))))

(fn CreateOrder)

(fn CheckonOrder
  (params (itemToCheck :type Integer))
  (if (> itemToCheck 0)
    (return true)))