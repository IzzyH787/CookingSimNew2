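; BP_LevelManager runs the restaurant game's levels, deciding when each of three levels is won or failed.
; BeginPlay initialises satisfaction and deadline values, counts BP_Chair actors and creates result widgets; Tick updates whether seating is full.
; Tick also checks the GameInstance's level number against completed orders, late orders or time limits, timed by raw GetRealTimeSeconds.
; Winning or failing shows its widget, switches to UI-only input and pauses the game.
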(event EventBeginPlay
  (Utilities|FlowControl|Sequence
    (:then_0
      ;[1 1 1] Initialise values
      (Variables|Default|SetcustomerSatisfaction 1e+02)
      (Variables|Default|SetorderDeadline 6e+02)
      (Variables|Default|SetcustomersSat 0))
    (:then_1
      ;[1 1 1] Count how many chairs in restaurant
      (bind _outactors (Actor|GetAllActorsOfClass "/Game/Blueprints/Furniture/BP_Chair.BP_Chair_C"))
      (for _array_element _outactors
        (Variables|Default|Setchairs (+ (Variables|Default|Getchairs) 1))))
    (:then_2
      ;[1 1 1] Create widget for when level is completed
      (bind _returnvalue (UserInterface|CreateWidget "/Game/UI/CAW_LevelComplete.CAW_LevelComplete_C"))
      (Variables|Default|SetLevelCompleteUI _returnvalue)
      ;[1 1 1] Create widgeth for when level is failed
      (bind _returnvalue_2 (UserInterface|CreateWidget "/Game/UI/CAW_LevelFailed.CAW_LevelFailed_C"))
      (Variables|Default|SetLevelFailedUI _returnvalue_2))))

(event EventTick
  (params (DeltaSeconds :type Float%20%28single-precision%29))
  (Utilities|FlowControl|Sequence
    (:then_0
      ;[1 1 1] Set restaurant full status
      (Variables|Default|SetrestaurantFull? (== (Variables|Default|GetcustomersSat) (Variables|Default|Getchairs))))
    (:then_1
      ;[1 0.3784 0.9388] Level 1 = Complete 10 Orders
      ;;[1 1 1] Check if first level
      (bind _matches_ (CallFunction|CheckLevelNumber))
      (if _matches_
        ;;[1 1 1] Check if 10 orders have been completed
        (if (>= (Variables|Default|GetordersCompleted) 1)
          (Variables|Default|SetlevelWon? true)
          (CallFunction|OpenCompleteMenu))))
    (:then_2
      ;[0.451 0.1081 1] Level 2 = complete 5 orders in 5 minutes
      ;;[1 1 1] Check if second level
      (bind _matches__2 (CallFunction|CheckLevelNumber 1))
      (if _matches__2
        (Variables|Default|SetlevelLength 2e+01)
        ;;[1 1 1] If still within time limit
        (bind _withinlimit_ (CallFunction|CheckifinTimeLimit (Utilities|Time|GetRealTimeSeconds)))
        (if _withinlimit_
          ;;[1 1 1] Checkif 5 orders completed
          (if (>= (Variables|Default|GetordersCompleted) 2)
            (CallFunction|OpenCompleteMenu))
          (else
            (Variables|Default|SetlevelWon? false)
            (CallFunction|OpenFailMenu)
            (Development|PrintText "Level Failed")))))
    (:then_3
      ;[0.009716 0 1] Level 3 = last 7 mns without having 3 late orders
      ;;[1 1 1] Check if third level
      (bind _matches__3 (CallFunction|CheckLevelNumber 2))
      (if _matches__3
        ;;[1 1 1] Level length = 15mins
        (Variables|Default|SetlevelLength 4.2e+02)
        ;;[1 1 1] Check if more than 10 orders have been completed late
        (if (>= (Variables|Default|GetlateOrdersCompleted) 3)
          ;;[1 1 1] Level failed
          (Variables|Default|SetlevelWon? false)
          (CallFunction|OpenFailMenu)
          (Development|PrintText "Level Failed")
          (else
            ;;[1 1 1] If still in time limit
            (bind _withinlimit__2 (CallFunction|CheckifinTimeLimit (Utilities|Time|GetRealTimeSeconds)))
            (if (not _withinlimit__2)
              ;;[1 1 1] Player has exceeded time limit without 10 -ive orders, win
              (Variables|Default|SetlevelWon? true)
              (CallFunction|OpenCompleteMenu))))))))

(event Input|KeyboardEvents|2
  (params (Key :type Key%20Structure :default "None"))
  (:Pressed
    (Variables|Default|SetlevelNumber 1)
    (Development|PrintString "level 2")))

(fn ConstructionScript)

(fn CheckLevel1Criteria)

(fn CheckifinTimeLimit
  (params (currentTime :type Float%20%28double-precision%29))
  (return (>= (Variables|Default|GetlevelLength) currentTime)))

(fn OpenCompleteMenu
  (bind _returnvalue (Game|GetPlayerController 0))
  (bind _levelcompleteui (Variables|Default|GetLevelCompleteUI))
  ;[1 1 1] Add UI to screen
  (Class|CommonActivatableWidget|ActivateWidget _levelcompleteui)
  (UserInterface|Viewport|AddtoViewport _levelcompleteui 0)
  ;[1 1 1] Change player controls
  (Input|SetInputModeUIOnly _returnvalue 0 "DoNotLock" false)
  (Variables|/Script/Engine.PlayerController|SetbShowMouseCursor _returnvalue true)
  ;[1 1 1] Stop gameplay of level
  (Game|SetGamePaused true))

(fn ChangeLevel
  (bind _asbp_game_instance (Utilities|Casting|CastToBP_GameInstance (Game|GetGameInstance)))
  (Variables|/Game/Blueprints/Non-physical/BP_GameInstance.BP_GameInstance_C|SetlevelNumber _asbp_game_instance (+ (Variables|/Game/Blueprints/Non-physical/BP_GameInstance.BP_GameInstance_C|GetlevelNumber _asbp_game_instance) 1)))

(fn CheckLevelNumber
  (params (checkValue :type Integer))
  (bind _asbp_game_instance (Utilities|Casting|CastToBP_GameInstance (Game|GetGameInstance)))
  (return (== (Variables|/Game/Blueprints/Non-physical/BP_GameInstance.BP_GameInstance_C|GetlevelNumber _asbp_game_instance) checkValue)))

(fn OpenFailMenu
  (bind _returnvalue (Game|GetPlayerController 0))
  (bind _levelfailedui (Variables|Default|GetLevelFailedUI))
  ;[1 1 1] Ad UI to screen
  (Class|CommonActivatableWidget|ActivateWidget _levelfailedui)
  (UserInterface|Viewport|AddtoViewport _levelfailedui 0)
  ;[1 1 1] Changing player controls
  (Input|SetInputModeUIOnly _returnvalue 0 "DoNotLock" false)
  (Variables|/Script/Engine.PlayerController|SetbShowMouseCursor _returnvalue true)
  ;[1 1 1] Stop gameplay of level
  (Game|SetGamePaused true))