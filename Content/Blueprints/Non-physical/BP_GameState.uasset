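; Game state Blueprint for an order-completion game, drafting win and fail rules for three levels based on orders completed, late orders and time limits.
; BeginPlay only creates and stores the level-complete widget, and Tick is empty.
; The rule sequence is disconnected and unfinished: only the first level's branch shows the widget and advances the level through BP_GameMode.
; CheckIfInTimeLimit is a stub that always returns false.
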(event EventTick
  (params (DeltaSeconds :type Float%20%28single-precision%29)))

(event EventBeginPlay
  ;[1 1 1] Create widget for when level is completed
  (bind _returnvalue (UserInterface|CreateWidget "/Game/UI/CAW_LevelComplete.CAW_LevelComplete_C"))
  (Variables|Default|SetLevelCompleteUI _returnvalue))

(fn ConstructionScript)

(fn CheckifinTimeLimit
  (params (currentTime :type Float%20%28double-precision%29))
  (return false))