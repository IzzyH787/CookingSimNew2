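; BP_Customer1 is a restaurant customer that walks to the till, then sits at an empty chair.
; Construction finds the "Till"-tagged target point and BeginPlay starts AI movement to it.
; Tick polls AtTill, waits, teleports the customer onto a free BP_Chair, updates BP_LevelManager's seated count and plays sitting animations.
; Player collisions trigger a shrug and reduce customer satisfaction, while a Handshake event plays an angry gesture.
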(event OnComponentHit(CapsuleComponent)
  (params (HitComponent :type Primitive%20Component%20Object%20Reference) (OtherActor :type Actor%20Object%20Reference) (OtherComp :type Primitive%20Component%20Object%20Reference) (NormalImpulse :type Vector :default "0, 0, 0") (Hit :type Hit%20Result%20Structure%20%28by%20ref%29))
  ;[1 1 1] If collides with player
  (if (Actor|ActorHasTag OtherActor "Player")
    (Utilities|FlowControl|Sequence
      (:then_0
        (Utilities|FlowControl|DoOnce false :!label _label
          (:Completed
            ;[1 1 1] Play shrug animation
            (Components|Animation|PlayAnimation (Variables|Character|GetMesh) "/Game/Characters/Models/Customer1/Shrugging.Shrugging" false)
            (Utilities|FlowControl|Delay 1.0)
            ;[1 1 1] Reset to animation bluepront
            (Components|Animation|PlayAnimation (Variables|Character|GetMesh) "/Game/Characters/Models/Customer1/Walking__4_.Walking__4_" true)
            (Components|Animation|SetAnimationMode (Variables|Character|GetMesh) "AnimationBlueprint")
            (goto _label Reset))))
      (:then_1
        (bind _returnvalue (Actor|GetActorOfClass "/Game/Blueprints/Non-physical/BP_LevelManager.BP_LevelManager_C"))
        (Variables|/Game/Blueprints/Non-physical/BP_LevelManager.BP_LevelManager_C|SetcustomerSatisfaction _returnvalue (- (Variables|/Game/Blueprints/Non-physical/BP_LevelManager.BP_LevelManager_C|GetcustomerSatisfaction _returnvalue) 5.0))))))

(event Custom|Handshake
  (Components|Animation|PlayAnimation (Variables|Character|GetMesh) "/Game/Characters/Models/Customer1/Angry_Gesture.Angry_Gesture" false))

(event EventBeginPlay
  ;[1 1 1] Make customer walk towards target point
  (AI|AIMoveTo self "0, 0, 0" (Variables|Default|GetTarget) 5.0 false))

(event EventTick
  (params (DeltaSeconds :type Float%20%28single-precision%29))
  (Utilities|FlowControl|Sequence
    (:then_0
      ;[1 1 1] Check if at till
      (if (Variables|Default|GetatTill?)
        (Variables|Default|SetatTill? false)
        ;[1 1 1] Create delay
        (Utilities|FlowControl|Delay 5.0)
        (Development|PrintString "Order complete")
        ;[1 1 1] Find empty chair
        (bind _outactors (Actor|GetAllActorsOfClass "/Game/Blueprints/Furniture/BP_Chair.BP_Chair_C"))
        (bind _array_element (Utilities|Array|ForEachLoopwithBreak _outactors :!label _label)
          (:LoopBody
            (if (Variables|/Game/Blueprints/Furniture/BP_Chair.BP_Chair_C|GetisEmpty _array_element)
              ;[1 1 1] Move player to chair
              (Transformation|SetActorLocation self (Math|Vector|MakeVector (.x (Transformation|GetActorLocation _array_element)) (.y (Transformation|GetActorLocation _array_element)) (+ (.z (Transformation|GetActorLocation _array_element)) 175.0)) false false)
              (Transformation|SetActorRotation self (Transformation|GetActorRotation _array_element))
              ;[1 1 1] Increment number of customers sat in restaurant
              (bind _returnvalue (Actor|GetActorOfClass "/Game/Blueprints/Non-physical/BP_LevelManager.BP_LevelManager_C"))
              (Variables|/Game/Blueprints/Non-physical/BP_LevelManager.BP_LevelManager_C|SetcustomersSat _returnvalue (+ (Variables|/Game/Blueprints/Non-physical/BP_LevelManager.BP_LevelManager_C|GetcustomersSat _returnvalue) 1))
              (Variables|/Game/Blueprints/Furniture/BP_Chair.BP_Chair_C|SetisEmpty _array_element false)
              (goto _label Break)))
          (:Completed
            (Utilities|FlowControl|DoOnce false
              (:Completed
                ;[1 1 1] Play shrug animation
                (Components|Animation|PlayAnimation (Variables|Character|GetMesh) "/Game/Characters/Models/Customer1/Stand_To_Sit.Stand_To_Sit" false)
                (Utilities|FlowControl|Delay 1.0)
                (Variables|Default|SetisSitting true)
                (Components|Animation|PlayAnimation (Variables|Character|GetMesh) "/Game/Characters/Models/Customer1/Male_Sitting_Pose.Male_Sitting_Pose" true)))))))))

(fn ConstructionScript
  (bind _outactors (Actor|GetAllActorsOfClass "/Script/Engine.TargetPoint"))
  (bind _array_element (Utilities|Array|ForEachLoopwithBreak _outactors)
    (:LoopBody
      (if (Actor|ActorHasTag _array_element "Till")
        (bind _output_get (Variables|Default|SetTarget _array_element))))))