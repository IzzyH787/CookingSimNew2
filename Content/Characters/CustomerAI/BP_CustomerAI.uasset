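; Customer AI character that varies its appearance and reacts when bumped by the player.
; The construction script randomizes top, trousers and skin materials and gives some customers glasses; the rare-afro hair roll is computed but never applied.
; On a player capsule hit while the blackboard "sat" flag is false, it plays a shrug, restores its AnimBP and lowers BP_LevelManager's customer satisfaction, with a delayed DoOnce reset throttling repeats.
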(event OnComponentHit(CapsuleComponent)
  (params (HitComponent :type Primitive%20Component%20Object%20Reference) (OtherActor :type Actor%20Object%20Reference) (OtherComp :type Primitive%20Component%20Object%20Reference) (NormalImpulse :type Vector :default "0, 0, 0") (Hit :type Hit%20Result%20Structure%20%28by%20ref%29))
  ;[1 1 1] If collides with player
  (if (and (Actor|ActorHasTag OtherActor "Player") (not (ScalableFloat|GetValueasBool (AI|GetBlackboard 0) (Utilities|Name|MakeLiteralName "sat"))))
    (Utilities|FlowControl|Sequence
      (:then_0
        (Utilities|FlowControl|DoOnce false :!label _label
          (:Completed
            ;[1 1 1] Play shrug animation
            (Components|Animation|PlayAnimation (Variables|Character|GetMesh) "/Game/Characters/Models/Customer1/Shrugging.Shrugging" false)
            (Utilities|FlowControl|Delay 1.0)
            ;[1 1 1] Reset to animation bluepront
            (Components|Animation|SetAnimationMode (Variables|Character|GetMesh) "AnimationBlueprint")
            ;[1 1 1] Deduct from customer satisfaction score
            (bind _returnvalue (Actor|GetActorOfClass "/Game/Blueprints/Non-physical/BP_LevelManager.BP_LevelManager_C"))
            (Variables|/Game/Blueprints/Non-physical/BP_LevelManager.BP_LevelManager_C|SetcustomerSatisfaction _returnvalue (- (Variables|/Game/Blueprints/Non-physical/BP_LevelManager.BP_LevelManager_C|GetcustomerSatisfaction _returnvalue) 5.0))
            (Utilities|FlowControl|Delay 1.0)
            (goto _label Reset)))))))

(fn ConstructionScript
  (Utilities|FlowControl|Sequence
    (:then_0
      (bind _material (CallFunction|ChoseClothesMaterial))
      ;[1 1 1] Set material of top
      (Rendering|Material|SetMaterial (Variables|Character|GetMesh) 8 _material))
    (:then_1
      (bind _material_2 (CallFunction|ChoseClothesMaterial))
      ;[1 1 1] Set material of trousers
      (Rendering|Material|SetMaterial (Variables|Character|GetMesh) 6 _material_2))
    (:then_2
      (bind _material_3 (CallFunction|ChoseifGlasses))
      ;[1 1 1] Set material of glasses
      (Rendering|Material|SetMaterial (Variables|Character|GetMesh) 4 _material_3))
    (:then_3
      (CallFunction|ChoseSkin))
    (:then_4
      (CallFunction|ChoseHair))))

(fn ChoseClothesMaterial
  ;[1 1 1] Chose random material
  (switch int (Math|Random|RandomIntegerinRange 0 12)
    (:0
      (bind _output_get (Variables|Default|SetTopMaterial "/Game/Characters/Models/Customer1/Wolf3D_Outfit_Top_005.Wolf3D_Outfit_Top_005"))
      (return _output_get))
    (:1
      (bind _output_get_2 (Variables|Default|SetTopMaterial "/Game/Materials/Colours/M_Black.M_Black"))
      (return _output_get_2))
    (:2
      (bind _output_get_3 (Variables|Default|SetTopMaterial "/Game/Materials/Colours/M_DarkRed.M_DarkRed"))
      (return _output_get_3))
    (:3
      (bind _output_get_4 (Variables|Default|SetTopMaterial "/Game/Assets/Cake/DarkBrown.DarkBrown"))
      (return _output_get_4))
    (:4
      (bind _output_get_5 (Variables|Default|SetTopMaterial "/Game/Assets/BeerBottle/DarkGreen.DarkGreen"))
      (return _output_get_5))
    (:5
      (bind _output_get_6 (Variables|Default|SetTopMaterial "/Game/Materials/Colours/M_PaleBlue.M_PaleBlue"))
      (return _output_get_6))
    (:6
      (bind _output_get_7 (Variables|Default|SetTopMaterial "/Game/Materials/Colours/M_Blue.M_Blue"))
      (return _output_get_7))
    (:7
      (bind _output_get_8 (Variables|Default|SetTopMaterial "/Game/Materials/Colours/M_Yellow.M_Yellow"))
      (return _output_get_8))
    (:8
      (bind _output_get_9 (Variables|Default|SetTopMaterial "/Game/Materials/Colours/M_Purple.M_Purple"))
      (return _output_get_9))
    (:9
      (bind _output_get_10 (Variables|Default|SetTopMaterial "/Game/Assets/BeerBottle/DarkGreen.DarkGreen"))
      (return _output_get_10))
    (:10
      (bind _output_get_11 (Variables|Default|SetTopMaterial "/Game/Materials/Colours/M_Brown.M_Brown"))
      (return _output_get_11))
    (:11
      (bind _output_get_12 (Variables|Default|SetTopMaterial "/Game/Materials/Colours/M_Black.M_Black"))
      (return _output_get_12))
    (:12
      (bind _output_get_13 (Variables|Default|SetTopMaterial "/Game/Materials/Colours/M_Green.M_Green"))
      (return _output_get_13))))

(fn ChoseifGlasses
  (if (<= (Math|Random|RandomIntegerinRange 0 100) 79)
    (return "/Engine/Functions/Engine_MaterialFunctions02/ExampleContent/3dParticleOpacity_Mat.3dParticleOpacity_Mat")
    (else
      (return "/Game/Characters/Models/Customer1/Wolf3D_Glasses_005.Wolf3D_Glasses_005"))))

(fn ChoseHair
  ;[1 1 1] 0.1% chance of customer having rainbow afro
  (if (== (Math|Random|RandomIntegerinRange 0 1000) 1)
    (return "/Game/Assets/Hairstyle1/hair.hair" "/Game/Assets/Hairstyle1/fredhair.fredhair")
    (else
      (return "/Engine/Functions/Engine_MaterialFunctions02/ExampleContent/3dParticleOpacity_Mat.3dParticleOpacity_Mat" "/Game/Assets/Hairstyle1/fredhair.fredhair"))))

(fn ChoseSkin
  (bind _mesh (Variables|Character|GetMesh))
  (bind _mesh_2 (Variables|Character|GetMesh))
  (bind _mesh_3 (Variables|Character|GetMesh))
  (switch int (Math|Random|RandomIntegerinRange 0 2)
    (:0
      (Rendering|Material|SetMaterial _mesh 1 "/Game/Materials/CustomerSkin/Tone1/M_Face1.M_Face1")
      (Rendering|Material|SetMaterial _mesh 5 "/Game/Materials/CustomerSkin/Tone1/M_Skin1.M_Skin1"))
    (:1
      (Rendering|Material|SetMaterial _mesh_2 1 "/Game/Materials/CustomerSkin/Tone2/M_Face2.M_Face2")
      (Rendering|Material|SetMaterial _mesh_2 5 "/Game/Materials/CustomerSkin/Tone2/M_Skin2.M_Skin2"))
    (:2
      (Rendering|Material|SetMaterial _mesh_3 1 "/Game/Materials/CustomerSkin/Tone3/M_Face3.M_Face3")
      (Rendering|Material|SetMaterial _mesh_3 5 "/Game/Materials/CustomerSkin/Tone3/M_Skin3.M_Skin3"))))